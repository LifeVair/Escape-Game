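; Lobby room of a VR game that stages the station alert, the computer's voice pitch and the player's exits to the next room and the finish screen.
; A timeline blends the lights into alert mode, switching status widgets and sounding the computer; reversing it restores the OK state.
; Standing at the PC triggers alert or pitch, which unlocks the room door trigger.
; Once the GameMode reports the game finished, the dome trigger sends the player to the finish screen.
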(event OnComponentBeginOverlap(Enteringtheroom)
  (params (OverlappedComponent :type Primitive%20Component%20Object%20Reference) (OtherActor :type Actor%20Object%20Reference) (OtherComp :type Primitive%20Component%20Object%20Reference) (OtherBodyIndex :type Integer) (bFromSweep :type Boolean) (SweepResult :type Hit%20Result%20Structure%20%28by%20ref%29))
  (bind _gamefinished (Default|GetGameFinished (Variables|Default|GetAs%20GM%20Main)))
  (if (Math|Boolean|ANDBoolean (not _gamefinished) (== OtherActor (Variables|Default|GetAs%20Life%20VR%20Character)) (Variables|Default|GetGame%20Ready))
    (Utilities|FlowControl|DoOnce false
      (:Completed
        ;[0.1979 0.1313 0 1 12] The player is teleported using a notify in the door animation !
        (Audio|Components|Audio|Play (Variables|Default|GetRoomDoor) false)
        (Variables|Default|SetInitialDoorOpening true)
        (Default|UpdateMusic (Variables|Default|GetAs%20GM%20Main) 2 true)))))

(event OnComponentBeginOverlap(InFrontOfThePC)
  (params (OverlappedComponent :type Primitive%20Component%20Object%20Reference) (OtherActor :type Actor%20Object%20Reference) (OtherComp :type Primitive%20Component%20Object%20Reference) (OtherBodyIndex :type Integer) (bFromSweep :type Boolean) (SweepResult :type Hit%20Result%20Structure%20%28by%20ref%29))
  (if (== OtherActor (Variables|Default|GetAs%20Life%20VR%20Character))
    (Variables|Default|SetInFrontOfPC true)
    (if (Variables|Default|GetAlertMode)
      (Utilities|FlowControl|DoOnce false
        (:Completed
          ;[0.5104 0.2768 0.3229] 🦜Pitch player
          (CallFunction|PitchPlayer)))
      (else
        (CallFunction|TurnLobbyAlertModeon)))))

(event OnComponentBeginOverlap(GameFinal-DomeDirection)
  (params (OverlappedComponent :type Primitive%20Component%20Object%20Reference) (OtherActor :type Actor%20Object%20Reference) (OtherComp :type Primitive%20Component%20Object%20Reference) (OtherBodyIndex :type Integer) (bFromSweep :type Boolean) (SweepResult :type Hit%20Result%20Structure%20%28by%20ref%29))
  (bind _gamefinished (Default|GetGameFinished (Variables|Default|GetAs%20GM%20Main)))
  (if (and _gamefinished (== OtherActor (Variables|Default|GetAs%20Life%20VR%20Character)))
    (Utilities|FlowControl|Delay 1.0)
    (Default|MovePlayertoFinishScreen (Variables|Default|GetAs%20GM%20Main) false)))

(event Custom|Simulate%20Player%20in%20Start%20Zone
  (Variables|Default|SetInFrontOfPC true)
  (if (Variables|Default|GetAlertMode)
    (Utilities|FlowControl|DoOnce false
      (:Completed
        ;[0.5104 0.2768 0.3229] 🦜Pitch player
        (CallFunction|PitchPlayer)))
    (else
      (CallFunction|TurnLobbyAlertModeon))))

(event Custom|Turn%20Lobby%20Alert%20mode%20on
  ;[0.1667 0.04427 0.04427] 🚨 Alert mode
  ;[0.005208 0.005208 0.005208] Keep environment visuals data for later
  (Utilities|FlowControl|DoOnce false
    (:Completed
      (Variables|EnvironmentControl|SetTopLight%20Base%20Intensity (Variables|/Script/Engine.LightComponentBase|GetIntensity (Variables|/Script/Engine.RectLight|GetRectLightComponent (Variables|EnvironmentControl|GetTopLight))))
      (Variables|EnvironmentControl|SetBottomLight%20Base%20Color (Rendering|Components|Light|GetLightColor (Variables|/Script/Engine.RectLight|GetRectLightComponent (Variables|EnvironmentControl|Getbottom_lights))))
      (bind (_direction _alpha) (Timeline|Color%20Animation Play)
        (:Update
          (Rendering|Components|Light|SetLightColor (Variables|/Script/Engine.RectLight|GetRectLightComponent (Variables|EnvironmentControl|Getbottom_lights)) (Math|Color|Lerp(LinearColor) (Variables|EnvironmentControl|GetBottomLight%20Base%20Color) (Variables|EnvironmentControl|GetAlert%20Bottom%20Light%20Color) _alpha) true)
          (Rendering|Components|Light|SetIntensity (Variables|/Script/Engine.RectLight|GetRectLightComponent (Variables|EnvironmentControl|GetTopLight)) (Math|Float|Lerp (Variables|EnvironmentControl|GetTopLight%20Base%20Intensity) (Variables|EnvironmentControl|GetTopLight%20Alert%20Intensity) _alpha)))
        (:Finished
          (switch Utilities|FlowControl|Switch|SwitchonETimelineDirection _direction
            (:Forward
              ;[0.005208 0.005208 0.005208] Alert Screen
              (Default|ShowAlertScreen (Variables|Default|GetAs%20WBP%20Rooms%20Status))
              (Default|GotoAlertScreen (Variables|Default|GetAs%20WBP%20Station%20Status))
              ;[0.005208 0.005208 0.005208] 📢 Play Alarm if far from PC
              (Audio|Components|Audio|Play (Variables|Default|GetComputer%20sound) 0.0)
              (if (Variables|Default|GetInFrontOfPC)
                (Utilities|FlowControl|Delay 2.0)
                (Variables|Default|SetAlertMode true)
                (Utilities|FlowControl|DoOnce false
                  (:Completed
                    ;[0.005208 0.005208 0.005208] Pitch Player
                    (CallFunction|PitchPlayer)))
                (else
                  (Variables|Default|SetAlertMode true))))
            (:Backward
              ;[0.005208 0.005208 0.005208] Green screen on computer
              (Default|ShowOkSituationScreen (Variables|Default|GetAs%20WBP%20Rooms%20Status))
              (Default|GotoOKScreen (Variables|Default|GetAs%20WBP%20Station%20Status))
              (Variables|Default|SetAlertMode false)
              ;[0.005208 0.005208 0.005208] Stop sound
              (Audio|Components|Audio|Stop (Variables|Default|GetComputer%20sound))
              (Audio|PlaySound2D "/Game/FX/SFCX/SFX/Cues/SC_MachineSucceeded.SC_MachineSucceeded" 1.0 1.0 0.0 0 0))))))))

(event Custom|Close%20Room%20Door
  (bind _roomdoor (Variables|Default|GetRoomDoor))
  ;[0.005208 0.005208 0.005208] Close  room door
  (Components|Timeline|SetPlayRate _roomdoor -1.0)
  (Audio|Components|Audio|Play _roomdoor false))

(event Custom|Recover%20Lobby%20State
  ;[0.02639 0.05729 0.01745] 🌱 Recover lobby
  (bind (_direction _alpha) (Timeline|Color%20Animation ReverseFromEnd)
    (:Update
      (Rendering|Components|Light|SetLightColor (Variables|/Script/Engine.RectLight|GetRectLightComponent (Variables|EnvironmentControl|Getbottom_lights)) (Math|Color|Lerp(LinearColor) (Variables|EnvironmentControl|GetBottomLight%20Base%20Color) (Variables|EnvironmentControl|GetAlert%20Bottom%20Light%20Color) _alpha) true)
      (Rendering|Components|Light|SetIntensity (Variables|/Script/Engine.RectLight|GetRectLightComponent (Variables|EnvironmentControl|GetTopLight)) (Math|Float|Lerp (Variables|EnvironmentControl|GetTopLight%20Base%20Intensity) (Variables|EnvironmentControl|GetTopLight%20Alert%20Intensity) _alpha)))
    (:Finished
      (switch Utilities|FlowControl|Switch|SwitchonETimelineDirection _direction
        (:Forward
          ;[0.005208 0.005208 0.005208] Alert Screen
          (Default|ShowAlertScreen (Variables|Default|GetAs%20WBP%20Rooms%20Status))
          (Default|GotoAlertScreen (Variables|Default|GetAs%20WBP%20Station%20Status))
          ;[0.005208 0.005208 0.005208] 📢 Play Alarm if far from PC
          (Audio|Components|Audio|Play (Variables|Default|GetComputer%20sound) 0.0)
          (if (Variables|Default|GetInFrontOfPC)
            (Utilities|FlowControl|Delay 2.0)
            (Variables|Default|SetAlertMode true)
            (Utilities|FlowControl|DoOnce false
              (:Completed
                ;[0.005208 0.005208 0.005208] Pitch Player
                (CallFunction|PitchPlayer)))
            (else
              (Variables|Default|SetAlertMode true))))
        (:Backward
          ;[0.005208 0.005208 0.005208] Green screen on computer
          (Default|ShowOkSituationScreen (Variables|Default|GetAs%20WBP%20Rooms%20Status))
          (Default|GotoOKScreen (Variables|Default|GetAs%20WBP%20Station%20Status))
          (Variables|Default|SetAlertMode false)
          ;[0.005208 0.005208 0.005208] Stop sound
          (Audio|Components|Audio|Stop (Variables|Default|GetComputer%20sound))
          (Audio|PlaySound2D "/Game/FX/SFCX/SFX/Cues/SC_MachineSucceeded.SC_MachineSucceeded" 1.0 1.0 0.0 0 0))))))

(event Custom|Open%20Dome%20Door
  (Development|PrintString "Open Dome Door" true true "(R=0.000000,G=0.964687,B=0.088656,A=1.000000)" 1e+01)
  (Audio|Components|Audio|Play (Variables|Default|GetDoor%20Dome) false)
  (Rendering|Material|SetScalarParameterValueonMaterials (Variables|Default|GetDoorWall%20Dome) "Blink Frequency" 1.0))

(event EventBeginPlay
  (CallFunction|DefineReferences)
  (Audio|Components|Audio|Stop (Variables|Default|GetComputer%20sound))
  (Class|GameplayStatics|SetBaseSoundMix "/Game/FX/SFCX/SoundMixes/SCM_Default.SCM_Default"))

(fn ConstructionScript)

(fn DefineReferences
  (bind _asgm_main (Utilities|Casting|CastToGM_Main (Game|GetGameMode)))
  (Variables|Default|SetAs%20GM%20Main _asgm_main)
  (bind _aswbp_station_status (Utilities|Casting|CastToWBP_StationStatus (UserInterface|GetWidget (Variables|Default|GetW_StationStatus))))
  (Variables|Default|SetAs%20WBP%20Station%20Status _aswbp_station_status)
  (bind _aswbp_rooms_status (Utilities|Casting|CastToWBP_RoomsStatus (UserInterface|GetWidget (Variables|Default|GetW_RoomStatus))))
  (Variables|Default|SetAs%20WBP%20Rooms%20Status _aswbp_rooms_status)
  (bind _aslife_vr_character (Utilities|Casting|CastToLife_VR_Character (Game|GetPlayerCharacter 0)))
  (Variables|Default|SetAs%20Life%20VR%20Character _aslife_vr_character))

(fn PitchPlayer
  (Default|GotoPitchScreen (Variables|Default|GetAs%20WBP%20Station%20Status))
  ;[0.005208 0.005208 0.005208] Pitch talking starts here
  (Audio|Components|Audio|SetSound (Variables|Default|GetComputer%20sound) "/Game/FX/SFCX/SFX/Cues/SC_VoicePitch.SC_VoicePitch")
  (Variables|Default|SetGame%20Ready true)
  ;[0.005208 0.005208 0.005208] Blink emissive of door room2 (Colour is red by default)
  (Rendering|Material|SetScalarParameterValueonMaterials (Variables|Default|GetDoorWall%20Room2) "Blink Frequency" 1.0))