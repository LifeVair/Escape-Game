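; Grippable pollutant tablet component for the lab room sorting puzzle, matched to snap areas by linked pollutant.
; Gripping lights it and highlights all BP_SnapArea zones; release snaps it into an overlapped free area, records correctness and fires TabletSnapped.
; Result events tint the emissive: success also locks gripping, failure restarts the Tick-driven sine blink.
; SnapTablet is an unwired leftover; TrySnap does the snapping.
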(event Custom|TabletWronglySorted
  (bind _fail_colour (Variables|Default|GetFail%20Colour))
  (Components|Tick|SetComponentTickEnabled true)
  (Development|PrintString "Tablet Sorting : Red Color" true true "(R=1.000000,G=0.000000,B=0.227560,A=1.000000)" 4.0)
  (Rendering|Material|SetVectorParameterValueonMaterials "Emissive_Color" (Math|Vector|MakeVector (.r _fail_colour) (.g _fail_colour) (.b _fail_colour))))

(event Custom|ToggleLedBlink
  (params (Blink%20On :type Boolean))
  (if Blink%20On
    (Components|Tick|SetComponentTickEnabled true)
    (else
      (Components|Tick|SetComponentTickEnabled false)
      (Rendering|Material|SetScalarParameterValueonMaterials "EmissiveStrength_Final" 0.0))))

(event Custom|Simulate%20Grip
  (bind _snappedarea (Variables|Default|GetSnappedArea))
  ;[0.005208 0.005208 0.005208] Disable blinking and light the tablet on grip
  (Components|Tick|SetComponentTickEnabled false)
  (Rendering|Material|SetScalarParameterValueonMaterials "EmissiveStrength_Final" 5.0)
  (CallFunction|SetIsSorted false)
  (bind _outactors (Actor|GetAllActorsOfClass "/Game/Core/Rooms/0_LabRoom/BP_SnapArea.BP_SnapArea_C"))
  (for _array_element _outactors
    (Default|HighlightZone _array_element)
    (Utilities|IsValid _snappedarea
      (:Is%20Valid
        (Default|SetAreaFilled _snappedarea false)))))

(event Custom|TabletCorrectlySorted
  (bind _success_colour (Variables|Default|GetSuccess%20Colour))
  (Development|PrintString "Tablet Sorting : GREEN Color" true true "(R=0.000000,G=1.000000,B=0.401192,A=1.000000)" 4.0)
  (Class|GrippableStaticMeshComponent|SetDenyGripping true)
  (Rendering|Material|SetVectorParameterValueonMaterials "Emissive_Color" (Math|Vector|MakeVector (.r _success_colour) (.g _success_colour) (.b _success_colour))))

(event Custom|Simulate%20Grip%20Release
  (bind _snapsucceeded (CallFunction|TrySnap))
  (if _snapsucceeded
    _
    (else
      (Development|PrintString "Tablet not snapped" true true "(R=1.000000,G=0.438805,B=0.000000,A=1.000000)" 12.0)))
  (bind _outactors (Actor|GetAllActorsOfClass "/Game/Core/Rooms/0_LabRoom/BP_SnapArea.BP_SnapArea_C"))
  (for _array_element _outactors
    (Default|StopZoneHighlight _array_element)))

(event EventSnap
  (params (Snap%20Transform :type Transform))
  (Transformation|SetWorldTransform (Math|Transform|MakeTransform (.location Snap%20Transform) (.rotation Snap%20Transform) (.scale Snap%20Transform)) false false)
  (Physics|SetSimulatePhysics false))

(event EventTick
  (params (DeltaSeconds :type Float%20%28single-precision%29))
  ;[0.005208 0.005208 0.005208 1 13] Enable by default to blink tablet in white before gipped
  ;[0.005208 0.005208 0.005208] Blink tablet emissive
  (bind _output_get (Variables|Default|SetCurrent%20time (+ (Variables|Default|GetCurrent%20time) DeltaSeconds)))
  (Rendering|Material|SetScalarParameterValueonMaterials "EmissiveStrength_Final" (* (Math|Trig|Sin(Degrees) (* _output_get (Variables|Default|GetBlink%20Frequency))) (Variables|Default|GetBlink%20Amplitude))))

(event EventOnGrip
  (params (GrippingController :type Grip%20Motion%20Controller%20Component%20Object%20Reference) (GripInformation :type BP%20Actor%20Grip%20Information%20Structure%20%28by%20ref%29))
  (bind _snappedarea (Variables|Default|GetSnappedArea))
  ;[0.005208 0.005208 0.005208] Disable blinking and light the tablet on grip
  (Components|Tick|SetComponentTickEnabled false)
  (Rendering|Material|SetScalarParameterValueonMaterials "EmissiveStrength_Final" 5.0)
  (CallFunction|SetIsSorted false)
  (bind _outactors (Actor|GetAllActorsOfClass "/Game/Core/Rooms/0_LabRoom/BP_SnapArea.BP_SnapArea_C"))
  (for _array_element _outactors
    (Default|HighlightZone _array_element)
    (Utilities|IsValid _snappedarea
      (:Is%20Valid
        (Default|SetAreaFilled _snappedarea false)))))

(event EventOnGripRelease
  (params (ReleasingController :type Grip%20Motion%20Controller%20Component%20Object%20Reference) (GripInformation :type BP%20Actor%20Grip%20Information%20Structure%20%28by%20ref%29) (bWasSocketed :type Boolean))
  (bind _snapsucceeded (CallFunction|TrySnap))
  (if _snapsucceeded
    _
    (else
      (Development|PrintString "Tablet not snapped" true true "(R=1.000000,G=0.438805,B=0.000000,A=1.000000)" 12.0)))
  (bind _outactors (Actor|GetAllActorsOfClass "/Game/Core/Rooms/0_LabRoom/BP_SnapArea.BP_SnapArea_C"))
  (for _array_element _outactors
    (Default|StopZoneHighlight _array_element)))

(event EventBeginPlay
  ;[0.005208 0.005208 0.005208] Keep lab room ref
  (bind _returnvalue (Actor|GetActorOfClass "/Game/Core/Rooms/0_LabRoom/BP_LabRoom.BP_LabRoom_C"))
  (Variables|Default|SetLabRoom _returnvalue)
  (CallFunction|ToggleLedBlink false))

(fn GetIsSorted
  (return (Variables|Default|GetisSorted)))

(fn SetIsSorted
  (params (Sorted :type Boolean))
  (Variables|Default|SetisSorted Sorted)
  (return))

(fn GetIsCorrectlySorted
  (return (Variables|Default|GetisCorrectlySorted)))

(fn SetIsCorrectlySorted
  (params (Correctly%20Sorted :type Boolean))
  (Variables|Default|SetisCorrectlySorted Correctly%20Sorted)
  (return))

(fn SnapTablet
  (params (Snapping%20Area :type BPI%20Snap%20Target%20Interface)))

(fn TrySnap
  (bind _outactors (Actor|GetAllActorsOfClass "/Game/Core/Rooms/0_LabRoom/BP_SnapArea.BP_SnapArea_C"))
  (bind _array_element (Utilities|Array|ForEachLoopwithBreak _outactors)
    (:LoopBody
      (if (!= (Utilities|Array|FindItem (Class|Actor|GetOverlappingComponents _array_element) self) -1)
        (bind _area_filled (Default|GetAreaFilled _array_element))
        (if _area_filled
          (Development|PrintString "Targeted Area already filled" true true "(R=1.000000,G=0.457758,B=0.000000,A=1.000000)" 1e+01)
          (else
            (LocalVariables|SetOverlapped%20Snap%20Area _array_element)))))
    (:Completed
      (Utilities|IsValid (LocalVariables|GetOverlapped%20Snap%20Area)
        (:Is%20Valid
          (CallFunction|Snap (Math|Transform|MakeTransform (.location (Transformation|GetWorldTransform (Variables|/Script/Engine.StaticMeshActor|GetStaticMeshComponent (LocalVariables|GetOverlapped%20Snap%20Area)))) (.rotation (Transformation|GetWorldTransform (Variables|/Script/Engine.StaticMeshActor|GetStaticMeshComponent (LocalVariables|GetOverlapped%20Snap%20Area)))) (Transformation|GetWorldScale self)))
          (Default|SetAreaFilled (LocalVariables|GetOverlapped%20Snap%20Area) true)
          (bind _output_get (Variables|Default|SetSnappedArea (LocalVariables|GetOverlapped%20Snap%20Area)))
          (Variables|Default|SetisSorted true)
          (CallFunction|SetIsCorrectlySorted (Utilities|Enum|Equal(Enum) (Variables|Default|GetLinkedPollutant) (Variables|/Game/Core/Rooms/0_LabRoom/BP_SnapArea.BP_SnapArea_C|GetLinkedPollutant _output_get)))
          (Default|CallTabletSnapped)
          (LocalVariables|SetOverlapped%20Snap%20Area 0)
          (return true))
        (:Is%20Not%20Valid
          (return false))))))