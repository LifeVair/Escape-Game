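; BP_SnapArea is a lab room snap zone that shows a visual highlight while it is available to be filled.
; HighlightZone unhides the static mesh only when AreaFilled is false, and StopZoneHighlight hides it again.
; A getter and setter expose AreaFilled, which is not changed by the highlight events, and both events print debug strings.
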(event EventStopZoneHighlight
  (Development|PrintString "Stop zone highlight" true true "(R=1.000000,G=0.554051,B=0.127857,A=1.000000)" 1e+01)
  (Development|SetHiddeninGame (Variables|Debug|GetStaticMeshComponent) true false))

(event EventHighlightZone
  (bind _debug (Variables|Default|GetDebug))
  (Development|PrintString "Highlighting zone" _debug _debug "(R=0.000000,G=0.660000,B=1.000000,A=1.000000)" 1e+01)
  (if (not (Variables|Default|GetAreaFilled))
    (Development|SetHiddeninGame (Variables|Debug|GetStaticMeshComponent) false false)))

(fn ConstructionScript)

(fn SetAreaFilled
  (params (Area%20Filled :type Boolean))
  (Variables|Default|SetAreaFilled Area%20Filled))

(fn GetAreaFilled
  (return (Variables|Default|GetAreaFilled)))