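; Lab-room analyzer station that accepts the filter cartridge and kicks off the room's puzzle.
; When the filter overlaps the box, a held filter is force-dropped, grip-locked and snapped to the cartridge socket.
; The alarm then stops, diagnostic screens play, tablets become grippable, lights come up and the GM_Main timer starts after a delay.
; FilterOk shows success on the screen widget and disables further overlap handling.
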(event OnComponentBeginOverlap(Box)
  (params (OverlappedComponent :type Primitive%20Component%20Object%20Reference) (OtherActor :type Actor%20Object%20Reference) (OtherComp :type Primitive%20Component%20Object%20Reference) (OtherBodyIndex :type Integer) (bFromSweep :type Boolean) (SweepResult :type Hit%20Result%20Structure%20%28by%20ref%29))
  (if (not (Variables|Default|GetRoomSucceeded))
    (if (== OtherComp (Variables|Default|GetLab%20Filter))
      (CallFunction|HandleFilterPlugged))))

(event Custom|Analyzing%20Filter
  (bind _analyzerscreen_ref (Variables|Default|GetAnalyzerScreen%20Ref))
  (Utilities|FlowControl|Sequence
    (:then_0
      ;[0.005208 0.005208 0.005208] Stop emissive
      (Rendering|Material|SetScalarParameterValueonMaterials (Variables|Default|GetStaticMesh) "EmissiveStrength_Final" 0.0))
    (:then_1
      (Utilities|FlowControl|Delay 3.0)
      (Default|ShowInstructions _analyzerscreen_ref))
    (:then_2
      (Default|ShowAnalysisScreen _analyzerscreen_ref)
      (Audio|PlaySoundatLocation "/Game/FX/Sounds/SFX/Cues/SC_FilterDiagnostic.SC_FilterDiagnostic" (Transformation|GetWorldLocation (Variables|Default|GetScreen)) "0, 0, 0" 1.0 1.0 0.0 "/Game/FX/Sounds/AttenuationSettings/SA_ElementCalling.SA_ElementCalling" 0 0 0))))

(event Custom|Handle%20Filter%20Plugged
  (bind _lab_filter (Variables|Default|GetLab%20Filter))
  (bind _lab_filter_2 (Variables|Default|GetLab%20Filter))
  (bind (_holdingcontrollers _bisheld) (Class|VRGripInterface|IsHeld _lab_filter))
  (if _bisheld
    (for _array_element _holdingcontrollers
      (bind _returnvalue (Class|GripMotionControllerComponent|DropObject (.holdingcontroller _array_element) _lab_filter (.gripid _array_element) false "0, 0, 0" "0, 0, 0"))
      (Development|PrintString "DROP OK" true true "(R=1.000000,G=0.260197,B=0.971056,A=1.000000)" 1e+01)
      (Class|GrippableStaticMeshComponent|SetDenyGripping _lab_filter true)
      (if _returnvalue
        (Development|PrintString "DropObject Filter Ok")
        (bind _returnvalue_2 (Transformation|AttachComponentToComponent _lab_filter_2 (Variables|Default|GetStaticMesh) "Cartridge Location" "SnapToTarget" "SnapToTarget" "KeepWorld" false))
        (if _returnvalue_2
          (Default|SetOriginRelativeTransform _lab_filter_2 (Transformation|GetWorldTransform _lab_filter_2))
          ;[0.005208 0.005208 0.005208] Stop alarm sound
          (Audio|Components|Audio|Stop (Variables|/Game/Core/Rooms/0_LabRoom/BP_LabRoom.BP_LabRoom_C|GetAudio (Variables|Default|GetLabRoom%20Ref)))
          ;[0.005208 0.005208 0.005208] Show game instruction and lock filter
          (CallFunction|AnalyzingFilter)
          (Utilities|FlowControl|Sequence
            (:then_0
              ;[0.005208 0.005208 0.005208] Start the timer after a certain amount of time
              (Utilities|FlowControl|Delay 1e+01)
              (bind _asgm_main (Utilities|Casting|CastToGM_Main (Game|GetGameMode)))
              (Default|StartTimer _asgm_main))
            (:then_1
              ;[0.005208 0.005208 0.005208] Enable tablet grip
              (for _array_element_2 (Actor|GetComponentsByClass (Variables|Default|GetLabRoom%20Ref) "/Game/Core/Rooms/0_LabRoom/BPC_PollutantTablet.BPC_PollutantTablet_C")
                (Class|GrippableStaticMeshComponent|SetDenyGripping _array_element_2 false)
                (Default|ToggleLedBlink _array_element_2 true))
              ;[0.0625 0.05108 0.006269] Light the room
              (Default|LighttheRoomUp (Variables|Default|GetLabRoom%20Ref)))))))
    (else
      (Audio|Components|Audio|Stop (Variables|/Game/Core/Rooms/0_LabRoom/BP_LabRoom.BP_LabRoom_C|GetAudio (Variables|Default|GetLabRoom%20Ref)))
      (CallFunction|AnalyzingFilter)
      (Utilities|FlowControl|Sequence
        (:then_0
          (Utilities|FlowControl|Delay 1e+01)
          (bind _asgm_main_2 (Utilities|Casting|CastToGM_Main (Game|GetGameMode)))
          (Default|StartTimer _asgm_main_2))
        (:then_1
          (for _array_element_3 (Actor|GetComponentsByClass (Variables|Default|GetLabRoom%20Ref) "/Game/Core/Rooms/0_LabRoom/BPC_PollutantTablet.BPC_PollutantTablet_C")
            (Class|GrippableStaticMeshComponent|SetDenyGripping _array_element_3 false)
            (Default|ToggleLedBlink _array_element_3 true))
          (Default|LighttheRoomUp (Variables|Default|GetLabRoom%20Ref)))))))

(event Custom|Filter%20Ok
  (Default|FilterOK (Variables|Default|GetAnalyzerScreen%20Ref))
  (Variables|Default|SetRoomSucceeded true))

(event EventBeginPlay
  (bind _returnvalue (Actor|GetActorOfClass "/Game/Core/Rooms/0_LabRoom/BP_LabRoom.BP_LabRoom_C"))
  (bind _output_get (Variables|Default|SetLabRoom%20Ref _returnvalue))
  (Variables|Default|SetLab%20Filter (Actor|GetComponentbyClass _output_get "/Game/Core/Rooms/0_LabRoom/BPC_Filter.BPC_Filter_C"))
  (bind _aswbp_analyzer_screen (Utilities|Casting|CastToWBP_AnalyzerScreen (UserInterface|GetWidget (Variables|Default|GetScreen))))
  (Variables|Default|SetAnalyzerScreen%20Ref _aswbp_analyzer_screen))

(fn ConstructionScript)