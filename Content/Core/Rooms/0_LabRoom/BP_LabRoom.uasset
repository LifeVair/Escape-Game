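; BP_LabRoom is the VR lab puzzle room where pollutant tablets are sorted to unlock a filter.
; Each tablet snap checks whether all are sorted, then marks each right or wrong; full success unlocks the filter and notifies BP_Analyzer.
; Overlapping the slot with the held filter force-drops and snaps it, ends the GM_Main timer and turns door emissives green.
; A SafeZone overlap respawns respawnable grippables.
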(event OnComponentBeginOverlap(FilterSlot)
  (params (OverlappedComponent :type Primitive%20Component%20Object%20Reference) (OtherActor :type Actor%20Object%20Reference) (OtherComp :type Primitive%20Component%20Object%20Reference) (OtherBodyIndex :type Integer) (bFromSweep :type Boolean) (SweepResult :type Hit%20Result%20Structure%20%28by%20ref%29))
  (bind _thelab (Variables|Default|GetTheLab))
  (bind _bp_filtercomponent (Variables|Default|GetBP_FilterComponent))
  (bind _pipe_filterslot (Variables|Default|GetPipe_FilterSlot))
  ;[0.005208 0.005208 0.005208 1 12] Execute the snapping mechanic only when game succeed
  (if (Variables|Default|GetFilterReadyToBePlugged)
    ;[0.005208 0.005208 0.005208] Snap filter to the slot
    (if (== OtherComp (Variables|Default|GetBP_FilterComponent))
      (bind (_holdingcontrollers _bisheld) (Class|VRGripInterface|IsHeld _bp_filtercomponent))
      (if _bisheld
        (for _array_element _holdingcontrollers
          (bind _returnvalue (Class|GripMotionControllerComponent|DropObject (.holdingcontroller _array_element) _bp_filtercomponent (.gripid _array_element) false "0, 0, 0" "0, 0, 0"))
          (Class|GrippableStaticMeshComponent|SetDenyGripping _bp_filtercomponent true)
          (if _returnvalue
            (Development|PrintString "DROp OK")
            (Transformation|AttachComponentToComponent _bp_filtercomponent _pipe_filterslot "Cartridge Location" "SnapToTarget" "SnapToTarget" "KeepWorld" false)
            ;[0.005208 0.005208 0.005208] Disable filter blink
            (Rendering|Material|SetMaterial _pipe_filterslot 0 "/Game/Assets/Props/Pipe_FilterSlot/MI_FilterSlot_NoBlink.MI_FilterSlot_NoBlink")
            (bind _asgm_main (Utilities|Casting|CastToGM_Main (Game|GetGameMode)))
            (Default|HandleTimerFinished _asgm_main true)
            ;[0.005208 0.005208 0.005208] Success color on door
            (Rendering|Material|SetVectorParameterValueonMaterials _thelab "Emissive_Color" "0.000000,1.000000,0.068000")
            (Rendering|Material|SetVectorParameterValueonMaterials _thelab "Emissive_NoiseRG_Speed" "0.052000,0.200000,0.000000")
            (Audio|PlaySoundatLocation "/Game/FX/Sounds/SFX/Cues/SC_RoomSucceed.SC_RoomSucceed" (Transformation|GetWorldLocation (Variables|Default|GetTheLab_Door)) "0, 0, 0" 1.0 1.0 0.0 "/Game/FX/Sounds/AttenuationSettings/SA_ElementCalling.SA_ElementCalling" 0 0 0)))))))

(event OnComponentBeginOverlap(SafeZone)
  (params (OverlappedComponent :type Primitive%20Component%20Object%20Reference) (OtherActor :type Actor%20Object%20Reference) (OtherComp :type Primitive%20Component%20Object%20Reference) (OtherBodyIndex :type Integer) (bFromSweep :type Boolean) (SweepResult :type Hit%20Result%20Structure%20%28by%20ref%29))
  (bind _asbpc_respawn_able_grippable (Utilities|Casting|CastToBPC_RespawnAbleGrippable OtherComp)
    (:then
      (Default|RespawnObject _asbpc_respawn_able_grippable))
    (:CastFailed
      (Development|PrintString "not a respawnable component"))))

(event Custom|Tablet%20Snapped
  (Variables|Default|SetAll%20Tablet%20Sorted true)
  (for _array_element (Actor|GetComponentsByClass "/Game/Core/Rooms/0_LabRoom/BPC_PollutantTablet.BPC_PollutantTablet_C")
    (bind _tablet_sorted (Default|GetIsSorted _array_element))
    (if (not _tablet_sorted)
      (Variables|Default|SetAll%20Tablet%20Sorted false)))
  (if (Variables|Default|GetAll%20Tablet%20Sorted)
    (bind _returnvalue (CallFunction|CheckRoomResult))
    (if _returnvalue
      ;[0.005208 0.005208 0.005208] Room Succeeded
      (Variables|Default|SetFilterReadyToBePlugged true)
      (Audio|PlaySoundatLocation "/Game/FX/Sounds/SFX/Cues/SC_MachineSucceeded.SC_MachineSucceeded" (Transformation|GetWorldLocation (Variables|Default|GetBP_Analyzer)) "0, 0, 0" 1.0 1.0 0.0 "/Game/FX/Sounds/AttenuationSettings/SA_ElementCalling.SA_ElementCalling" 0 0 0)
      ;[0.005208 0.005208 0.005208] Unlock filter
      (Class|Room|UnlockKey)
      (else
        (Audio|PlaySound2D "/Engine/EditorSounds/Notifications/CompileFailed_Cue.CompileFailed_Cue" 1.0 1.0 0.0 0 0 false)))))

(event Custom|Light%20The%20Room%20Up
  (Rendering|Components|Light|SetIntensity (Variables|Default|GetRectLight) 5.0))

(event Custom|UnlitPathToFilter
  (Rendering|Material|SetScalarParameterValueonMaterials (Variables|Default|GetTheLab) "EmissiveStrength_Final" 0.0))

(event Custom|Simulate%20Handle%20Filter%20Plugged%20success
  (bind _thelab (Variables|Default|GetTheLab))
  ;[0.005208 0.005208 0.005208] Disable filter blink
  (Rendering|Material|SetMaterial (Variables|Default|GetPipe_FilterSlot) 0 "/Game/Assets/Props/Pipe_FilterSlot/MI_FilterSlot_NoBlink.MI_FilterSlot_NoBlink")
  (bind _asgm_main (Utilities|Casting|CastToGM_Main (Game|GetGameMode)))
  (Default|HandleTimerFinished _asgm_main true)
  ;[0.005208 0.005208 0.005208] Success color on door
  (Rendering|Material|SetVectorParameterValueonMaterials _thelab "Emissive_Color" "0.000000,1.000000,0.068000")
  (Rendering|Material|SetVectorParameterValueonMaterials _thelab "Emissive_NoiseRG_Speed" "0.052000,0.200000,0.000000")
  (Audio|PlaySoundatLocation "/Game/FX/Sounds/SFX/Cues/SC_RoomSucceed.SC_RoomSucceed" (Transformation|GetWorldLocation (Variables|Default|GetTheLab_Door)) "0, 0, 0" 1.0 1.0 0.0 "/Game/FX/Sounds/AttenuationSettings/SA_ElementCalling.SA_ElementCalling" 0 0 0))

(event EventBeginPlay
  (Rendering|Components|Light|SetIntensity (Variables|Default|GetRectLight) 1.0)
  (for _array_element (Actor|GetComponentsByClass "/Game/Core/Rooms/BPC_RespawnAbleGrippable.BPC_RespawnAbleGrippable_C")
    (Default|SetOriginRelativeTransform _array_element (Transformation|GetRelativeTransform _array_element))
    (for _array_element_2 (Actor|GetComponentsByClass "/Game/Core/Rooms/0_LabRoom/BPC_PollutantTablet.BPC_PollutantTablet_C")
      (EventDispatchers|BindEventtoTabletSnapped _array_element_2 (delegate Custom|Tablet%20Snapped))
      (Class|GrippableStaticMeshComponent|SetDenyGripping _array_element_2 true))))

(event EventUnlockKey
  (Class|GrippableStaticMeshComponent|SetDenyGripping (Variables|Default|GetBP_FilterComponent) false)
  (bind _returnvalue (Actor|GetActorOfClass "/Game/Core/Rooms/0_LabRoom/BP_Analyzer.BP_Analyzer_C"))
  (Default|FilterOk _returnvalue))

(fn ConstructionScript
  (Components|Movement|SetUpdatedComponent (Variables|Default|GetFanRotation) (Variables|Default|GetFan)))

(fn CheckRoomResult
  ;[0 0 0 1 12] Initiate at true and change the result depending on the sorting results
  (Variables|Default|SetTabletsCorrectlySorted true)
  (for _array_element (Actor|GetComponentsByClass "/Game/Core/Rooms/0_LabRoom/BPC_PollutantTablet.BPC_PollutantTablet_C")
    (bind _tablet_correctly_sorted (Default|GetIsCorrectlySorted _array_element))
    (if _tablet_correctly_sorted
      (Default|TabletCorrectlySorted _array_element)
      (else
        (Default|TabletWronglySorted _array_element)
        (Variables|Default|SetTabletsCorrectlySorted false))))
  (return (Variables|Default|GetTabletsCorrectlySorted)))