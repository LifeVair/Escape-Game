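; BP_CO2Globe is a Lab Room CO2 demonstration device with a spinning globe and a gas bottle opened by a screw dial.
; Tick yaws the globe continuously.
; Turning the screw to at least 90 degrees opens the bottle once, playing a gas-release sound and disabling further gripping.
; A timeline then ramps the CO2 particle spawn rate and the temperature widget's progress bar together.
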(event OnDialHitSnapAngle(Screw)
  (params (DialMilestoneAngle :type Float%20%28single-precision%29))
  (if (>= DialMilestoneAngle 9e+01)
    (Utilities|FlowControl|DoOnce false
      (:Completed
        (CallFunction|BottleOpened)))))

(event Custom|Fill%20device%20with%20CO2
  ;[0.005208 0.005208 0.005208 1 12] Fill the atmosphere with pparticles and update temperature
  (bind _aswbp_temperature (Utilities|Casting|CastToWBP_Temperature (UserInterface|GetWidget (Variables|Default|GetWidget))))
  (bind _alpha (Timeline|Timeline Play)
    (:Update
      (Default|FillProgressBar _aswbp_temperature (Math|Float|Lerp 0.2 0.85 _alpha))
      (Effects|Components|ParticleSystem|SetFloatParameter (Variables|Default|GetCO2Globe) "Spawn Rate" (Math|Float|Lerp 0.0 2e+02 _alpha)))))

(event Custom|BottleOpened
  (Development|PrintString "Bottle Opened" true true "(R=1.000000,G=0.000000,B=0.626402,A=1.000000)" 5.0)
  (Audio|PlaySoundatLocation "/Game/FX/SFCX/SFX/Cues/SC_GasRelease.SC_GasRelease" (Variables|/Script/Engine.SceneComponent|GetRelativeLocation (Variables|Default|GetScrew)) "0, 0, 0" 1.0 1.0 0.0 0 0 0 0)
  (CallFunction|FillDevicewithCO2)
  (Variables|/Script/VRExpansionPlugin.VRDialComponent|SetbDenyGripping (Variables|Default|GetScrew) true))

(event EventTick
  (params (DeltaSeconds :type Float%20%28single-precision%29))
  (bind _globe (Variables|Default|GetGlobe))
  (bind _relativerotation (Variables|/Script/Engine.SceneComponent|GetRelativeRotation _globe))
  (bind (_roll _pitch _yaw) (Math|Rotator|BreakRotator _relativerotation))
  (Transformation|SetRelativeRotation _globe (Math|Rotator|MakeRotator _roll _pitch (+ _yaw (* DeltaSeconds 45.0))) false false))

(fn ConstructionScript)