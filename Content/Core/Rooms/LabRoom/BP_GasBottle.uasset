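; BP_GasBottle is a lab-room gas bottle that the player opens by turning its Screw dial to release CO2.
; Snap-angle and lerp-finished events from the dial share a check that opens the bottle once the milestone angle reaches the threshold.
; Opening plays a gas sound at the Screw's relative location, tells the BP_CO2Globe found by class to fill with CO2, and denies further gripping.
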(event OnDialHitSnapAngle(Screw)
  (params (DialMilestoneAngle :type Float%20%28single-precision%29))
  (if (>= DialMilestoneAngle 6e+01)
    (Utilities|FlowControl|DoOnce false
      (:Completed
        (CallFunction|BottleOpened)))))

(event OnDialFinishedLerping(Screw)
  (Development|PrintString "Finish lerping" true true "(R=0.000000,G=0.660000,B=1.000000,A=1.000000)" 5.0)
  (if (>= (stale OnDialHitSnapAngle(Screw) DialMilestoneAngle) 6e+01)
    (Utilities|FlowControl|DoOnce false
      (:Completed
        (CallFunction|BottleOpened)))))

(event Custom|BottleOpened
  (Development|PrintString "Bottle Opened" true true "(R=1.000000,G=0.000000,B=0.626402,A=1.000000)" 5.0)
  (Audio|PlaySoundatLocation "/Game/FX/SFCX/SFX/Cues/SC_GasRelease.SC_GasRelease" (Variables|/Script/Engine.SceneComponent|GetRelativeLocation (Variables|Default|GetScrew)) "0, 0, 0" 1.0 1.0 0.0 0 0 0 0)
  (bind _returnvalue (Actor|GetActorOfClass "/Game/Core/Rooms/LabRoom/BP_CO2Globe.BP_CO2Globe_C"))
  (Default|FillDevicewithCO2 _returnvalue)
  (Variables|/Script/VRExpansionPlugin.VRDialComponent|SetbDenyGripping (Variables|Default|GetScrew) true))

(fn ConstructionScript)