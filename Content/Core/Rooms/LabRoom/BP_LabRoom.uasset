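; VR lab puzzle room where the player sorts pollutant tablets to unlock a filter, then plugs it in before time runs out.
; Tablet snap events trigger a sorting check; success frees the filter, which auto-drops and attaches on overlapping its slot.
; Plugging it stops the GM_Main timer and opens the door, whose trigger returns the player to the lobby.
; The timer also drives Niagara gas density, and a safe zone respawns stray grippables.
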(event OnComponentBeginOverlap(FilterSlot)
  (params (OverlappedComponent :type Primitive%20Component%20Object%20Reference) (OtherActor :type Actor%20Object%20Reference) (OtherComp :type Primitive%20Component%20Object%20Reference) (OtherBodyIndex :type Integer) (bFromSweep :type Boolean) (SweepResult :type Hit%20Result%20Structure%20%28by%20ref%29))
  (bind _door (Variables|Default|GetDoor))
  (bind _bp_filtercomponent (Variables|Default|GetBP_FilterComponent))
  (bind _pipe_filterslot (Variables|Default|GetPipe_FilterSlot))
  ;[0.005208 0.005208 0.005208 1 12] Execute the snapping mechanic only when game succeed
  (if (Variables|Default|GetFilterReadyToBePlugged)
    ;[0.005208 0.005208 0.005208] Snap filter to the slot
    (if (== OtherComp (Variables|Default|GetBP_FilterComponent))
      (bind (_holdingcontrollers _bisheld) (Class|VRGripInterface|IsHeld _bp_filtercomponent))
      (if _bisheld
        (for _array_element _holdingcontrollers
          (bind _returnvalue (Class|GripMotionControllerComponent|DropObject (.holdingcontroller _array_element) _bp_filtercomponent (.gripid _array_element) false "0, 0, 0" "0, 0, 0"))
          (Class|GrippableStaticMeshComponent|SetDenyGripping _bp_filtercomponent true)
          (if _returnvalue
            (Development|PrintString "DROp OK")
            (Transformation|AttachComponentToComponent _bp_filtercomponent _pipe_filterslot "Cartridge Location" "SnapToTarget" "SnapToTarget" "KeepWorld" false)
            ;[0.005208 0.005208 0.005208] Disable filter blink
            (Rendering|Material|SetMaterial _pipe_filterslot 0 "/Game/Assets/Props/Pipe_FilterSlot/MI_FilterSlot_NoBlink.MI_FilterSlot_NoBlink")
            (bind _asgm_main (Utilities|Casting|CastToGM_Main (Game|GetGameMode)))
            ;[0 0.9647 0.08866] Timer success mode
            (Default|HandleTimerFinished _asgm_main true)
            ;[0.005208 0.005208 0.005208] Play door animation
            ;;[0.005208 0.005208 0.005208] Success color on door
            (Rendering|Material|SetVectorParameterValueonMaterials _door "Emissive_Color" "0.058845,0.760417,0.000000")
            (Audio|PlaySoundatLocation "/Game/FX/SFCX/SFX/Cues/SC_RoomSucceed.SC_RoomSucceed" (Transformation|GetWorldLocation _door) "0, 0, 0" 1.0 1.0 0.0 "/Game/FX/SFCX/AttenuationSettings/SA_ElementCalling.SA_ElementCalling" 0 0 0)
            (Audio|Components|Audio|Play _door false)
            (Variables|Default|SetRoomValidated true)))))))

(event OnComponentBeginOverlap(SafeZone)
  (params (OverlappedComponent :type Primitive%20Component%20Object%20Reference) (OtherActor :type Actor%20Object%20Reference) (OtherComp :type Primitive%20Component%20Object%20Reference) (OtherBodyIndex :type Integer) (bFromSweep :type Boolean) (SweepResult :type Hit%20Result%20Structure%20%28by%20ref%29))
  (bind _asbpc_respawn_able_grippable (Utilities|Casting|CastToBPC_RespawnAbleGrippable OtherComp)
    (:then
      (Default|RespawnObject _asbpc_respawn_able_grippable))
    (:CastFailed
      (Development|PrintString "not a respawnable component"))))

(event OnComponentBeginOverlap(Box)
  (params (OverlappedComponent :type Primitive%20Component%20Object%20Reference) (OtherActor :type Actor%20Object%20Reference) (OtherComp :type Primitive%20Component%20Object%20Reference) (OtherBodyIndex :type Integer) (bFromSweep :type Boolean) (SweepResult :type Hit%20Result%20Structure%20%28by%20ref%29))
  ;[0.005208 0.005208 0.005208] Front door area detection
  (if (Variables|Default|GetRoomValidated)
    (Utilities|FlowControl|Delay 1.0)
    ;[0.005208 0.005208 0.005208] Send back player to lobby
    (bind _asgm_main (Utilities|Casting|CastToGM_Main (Game|GetGameMode)))
    (Default|RecoverLobbyState (Variables|/Game/Core/GM_Main.GM_Main_C|GetLobby _asgm_main))
    (Default|MovePlayeratTargetArrow _asgm_main (Variables|/Game/Core/Rooms/Lobby/BP_LobbyRoom.BP_LobbyRoom_C|GetPlayerReturn (Variables|/Game/Core/GM_Main.GM_Main_C|GetLobby _asgm_main)))
    (Default|UpdateMusic _asgm_main 0 false)
    (Default|CloseRoomDoor (Variables|/Game/Core/GM_Main.GM_Main_C|GetLobby _asgm_main))
    (Utilities|FlowControl|Delay 1.5)
    (Default|OpenDomeDoor (Variables|/Game/Core/GM_Main.GM_Main_C|GetLobby _asgm_main))))

(event Custom|Tablet%20Snapped
  ;[0.005208 0.005208 0.005208] Tablet snapped
  (Variables|Default|SetAll%20Tablet%20Sorted true)
  (for _array_element (Actor|GetComponentsByClass "/Game/Core/Rooms/LabRoom/BPC_PollutantTablet.BPC_PollutantTablet_C")
    (bind _tablet_sorted (Default|GetIsSorted _array_element))
    (if (not _tablet_sorted)
      (Variables|Default|SetAll%20Tablet%20Sorted false)))
  (if (Variables|Default|GetAll%20Tablet%20Sorted)
    (bind _returnvalue (CallFunction|CheckRoomResult))
    (if _returnvalue
      ;;[0 0.3646 0.00132] Room Succeeded
      (Variables|Default|SetFilterReadyToBePlugged true)
      (Audio|PlaySoundatLocation "/Game/FX/SFCX/SFX/Cues/SC_MachineSucceeded.SC_MachineSucceeded" (Transformation|GetWorldLocation (Variables|Default|GetBP_Analyzer)) "0, 0, 0" 1.0 1.0 0.0 "/Game/FX/SFCX/AttenuationSettings/SA_ElementCalling.SA_ElementCalling" 0 0 0)
      ;;[0.005208 0.005208 0.005208] Unlock filter
      (Class|Room|UnlockKey)
      (else
        (Audio|PlaySound2D "/Engine/EditorSounds/Notifications/CompileFailed_Cue.CompileFailed_Cue" 1.0 1.0 0.0 0 0 false)))))

(event Custom|Light%20The%20Room%20Up
  ;[0.2344 0.1899 0.0729] 💡 Light the room up
  (Development|SetHiddeninGame (Variables|Default|GetSpotLight) true false)
  (bind _alpha (Timeline|Lighting Play)
    (:Update
      ;[0.005208 0.005208 0.005208] set light intensity
      (Rendering|Components|Light|SetIntensity (Variables|Default|GetRectLight) (Math|Float|Lerp 0.0 (Variables|Default|GetLight%20Emissive%20Strength) _alpha)))
    (:Finished
      ;[0.005208 0.005208 0.005208] Enable pollutants niagara particles in the chamber
      (for _array_element (Actor|GetComponentsbyTag "/Script/Niagara.NiagaraComponent" "ChamberPollutants")
        (Components|Activation|SetActive _array_element true false)))))

(event Custom|UnlitPathToFilter)

(event Custom|Simulate%20Handle%20Filter%20Plugged%20success
  (bind _door (Variables|Default|GetDoor))
  ;[0.005208 0.005208 0.005208] Disable filter blink
  (Rendering|Material|SetMaterial (Variables|Default|GetPipe_FilterSlot) 0 "/Game/Assets/Props/Pipe_FilterSlot/MI_FilterSlot_NoBlink.MI_FilterSlot_NoBlink")
  (bind _asgm_main (Utilities|Casting|CastToGM_Main (Game|GetGameMode)))
  ;[0 0.9647 0.08866] Timer success mode
  (Default|HandleTimerFinished _asgm_main true)
  ;[0.005208 0.005208 0.005208] Play door animation
  ;;[0.005208 0.005208 0.005208] Success color on door
  (Rendering|Material|SetVectorParameterValueonMaterials _door "Emissive_Color" "0.058845,0.760417,0.000000")
  (Audio|PlaySoundatLocation "/Game/FX/SFCX/SFX/Cues/SC_RoomSucceed.SC_RoomSucceed" (Transformation|GetWorldLocation _door) "0, 0, 0" 1.0 1.0 0.0 "/Game/FX/SFCX/AttenuationSettings/SA_ElementCalling.SA_ElementCalling" 0 0 0)
  (Audio|Components|Audio|Play _door false)
  (Variables|Default|SetRoomValidated true))

(event Custom|Simulate%20success
  (bind _door (Variables|Default|GetDoor))
  (bind _asgm_main (Utilities|Casting|CastToGM_Main (Game|GetGameMode)))
  ;[0 0.9647 0.08866] Timer success mode
  (Default|HandleTimerFinished _asgm_main true)
  ;[0.005208 0.005208 0.005208] Play door animation
  ;;[0.005208 0.005208 0.005208] Success color on door
  (Rendering|Material|SetVectorParameterValueonMaterials _door "Emissive_Color" "0.058845,0.760417,0.000000")
  (Audio|PlaySoundatLocation "/Game/FX/SFCX/SFX/Cues/SC_RoomSucceed.SC_RoomSucceed" (Transformation|GetWorldLocation _door) "0, 0, 0" 1.0 1.0 0.0 "/Game/FX/SFCX/AttenuationSettings/SA_ElementCalling.SA_ElementCalling" 0 0 0)
  (Audio|Components|Audio|Play _door false)
  (Variables|Default|SetRoomValidated true))

(event Custom|OnTimerUpdate_Event
  (params (TimerMinutes :type Integer) (TimerSecondes :type Integer))
  (CallFunction|HandleGameTimer TimerMinutes TimerSecondes))

(event EventBeginPlay
  (bind _asgm_main (Utilities|Casting|CastToGM_Main (Game|GetGameMode)))
  ;[0.005208 0.005208 0.005208 1 12] light room down
  (Rendering|Components|Light|SetIntensity (Variables|Default|GetRectLight) 0.2)
  (EventDispatchers|AssignOnTimerUpdate _asgm_main (delegate Custom|OnTimerUpdate_Event))
  (for _array_element (Actor|GetComponentsByClass self "/Game/Core/Rooms/BPC_RespawnAbleGrippable.BPC_RespawnAbleGrippable_C")
    (Default|SetOriginRelativeTransform _array_element (Transformation|GetWorldTransform _array_element)))
  (for _array_element_2 (Actor|GetComponentsByClass "/Game/Core/Rooms/LabRoom/BPC_PollutantTablet.BPC_PollutantTablet_C")
    (EventDispatchers|BindEventtoTabletSnapped _array_element_2 (delegate Custom|Tablet%20Snapped))
    (Class|GrippableStaticMeshComponent|SetDenyGripping _array_element_2 true)))

(event EventUnlockKey
  (Class|GrippableStaticMeshComponent|SetDenyGripping (Variables|Default|GetBP_FilterComponent) false)
  (bind _returnvalue (Actor|GetActorOfClass "/Game/Core/Rooms/LabRoom/BP_Analyzer.BP_Analyzer_C"))
  (Default|FilterOk _returnvalue))

(fn ConstructionScript)

(fn CheckRoomResult
  ;[0 0 0 1 12] Initiate at true and change the result depending on the sorting results
  (Variables|Default|SetTabletsCorrectlySorted true)
  (for _array_element (Actor|GetComponentsByClass "/Game/Core/Rooms/LabRoom/BPC_PollutantTablet.BPC_PollutantTablet_C")
    (bind _tablet_correctly_sorted (Default|GetIsCorrectlySorted _array_element))
    (if _tablet_correctly_sorted
      (Default|TabletCorrectlySorted _array_element)
      (else
        (Default|TabletWronglySorted _array_element)
        (Variables|Default|SetTabletsCorrectlySorted false))))
  (return (Variables|Default|GetTabletsCorrectlySorted)))

(fn HandleGameTimer
  (params (Minutes :type Integer) (Seconds :type Integer))
  (bind _output_get (LocalVariables|SetRemainingSeconds (+ (* Minutes 60) Seconds)))
  (Niagara|SetNiagaraVariable(Float) (Variables|Default|GetGaz) "AlphaSpawnRate" (Math|Float|Lerp 1.0 0.0 (/ _output_get (* (Variables|Default|GetAvailableTimeToResolve) 60)))))