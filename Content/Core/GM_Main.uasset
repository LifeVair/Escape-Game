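; Main game mode for a VR escape-room game, managing save data, room sessions and the room countdown.
; On BeginPlay it caches the VR character and loads or creates the persistent save object.
; New sessions spawn a room, take its time limit, teleport the player to its spawn and bind room success, which currently only logs.
; A looping one-second timer updates the character's countdown; save loading and room selection are unfinished.
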(event EventBeginPlay
  (bind _generalgm_debug (Variables|DEBUG|GetGeneralGM%20Debug))
  (bind _aslife_vr_character (Utilities|Casting|CastToLife_VR_Character (Game|GetPlayerCharacter 0))
    (:then
      (Variables|Default|SetAs%20Life%20VR%20Character _aslife_vr_character))
    (:CastFailed
      _))
  ;[1 0.3072 0 1 14] Load persistent data to a variable
  (bind _returnvalue (SaveGame|LoadGamefromSlot "PersistantData"))
  (bind _asbp_escape_game_save (Utilities|Casting|CastToBP_EscapeGameSave _returnvalue)
    (:then
      (Development|PrintString "Loading Game Settings ok" _generalgm_debug _generalgm_debug "(R=0.211777,G=0.596354,B=0.000000,A=1.000000)" 8.0 "GameSettingsLoad")
      (Variables|GameSave|SetSaveData _asbp_escape_game_save))
    (:CastFailed
      (Development|PrintString "Loading Game Settings Failed" _generalgm_debug _generalgm_debug "(R=0.828125,G=0.357734,B=0.000000,A=1.000000)" 8.0 "GameSettingsLoad")
      (bind _returnvalue_2 (SaveGame|CreateSaveGameObject "/Game/Core/SaveManager/BP_EscapeGameSave.BP_EscapeGameSave_C"))
      (Variables|GameSave|SetSaveData _returnvalue_2))))

(event Custom|Handle%20Timer%20Finished
  (params (Success :type Boolean))
  (bind _as_life_vr_character (Variables|Default|GetAs%20Life%20VR%20Character))
  ;[0.005208 0.005208 0.005208] Timer finished
  (Development|PrintString "TIMER STOPPED" true true "(R=0.000000,G=0.660000,B=1.000000,A=1.000000)" 2.0 "Timer")
  (Utilities|Time|ClearandInvalidateTimerbyHandle (Variables|TimerManagement|GetTimer))
  (Utilities|IsValid _as_life_vr_character
    (:Is%20Valid
      (Default|TimerFinished _as_life_vr_character Success))))

(event Custom|Start%20Timer
  (bind _as_life_vr_character (Variables|Default|GetAs%20Life%20VR%20Character))
  ;[0.005208 0.005208 0.005208] Timer Start
  (bind _returnvalue (Utilities|Time|SetTimerbyEvent (delegate Custom|Handle%20Timer%20Update) 1.0 true))
  (Variables|TimerManagement|SetTimer _returnvalue)
  (Utilities|IsValid _as_life_vr_character
    (:Is%20Valid
      (Default|TimerStart _as_life_vr_character))))

(event Custom|Handle%20Timer%20Update
  (bind _as_life_vr_character (Variables|Default|GetAs%20Life%20VR%20Character))
  ;[0.005208 0.005208 0.005208] Timer Update
  (Utilities|FlowControl|Sequence
    (:then_0
      (Development|PrintString "Update Timer value" true true "(R=0.000000,G=0.660000,B=1.000000,A=1.000000)" 2.0 "UpdateTimerValue")
      ;[0 0 0] Update Timer Value
      (if (== (Variables|TimerManagement|GetTimerSeconds) 0)
        (if (== (Variables|TimerManagement|GetTimerMinutes) 0)
          (CallFunction|HandleTimerFinished false)
          (else
            (Math|Integer|DecrementInt (Variables|TimerManagement|GetTimerMinutes)
              (:%20%20
                (Variables|TimerManagement|SetTimerSeconds 59)))))
        (else
          (Math|Integer|DecrementInt (Variables|TimerManagement|GetTimerSeconds)))))
    (:then_1
      (Utilities|IsValid _as_life_vr_character
        (:Is%20Valid
          (Default|UpdateTimer _as_life_vr_character (Variables|TimerManagement|GetTimerMinutes) (Variables|TimerManagement|GetTimerSeconds)))))))

(event Custom|Resume%20Timer
  (Utilities|Time|UnpauseTimerbyHandle (Variables|TimerManagement|GetTimer)))

(event Custom|Pause%20Timer
  (Utilities|Time|PauseTimerbyHandle (Variables|TimerManagement|GetTimer)))

(fn ConstructionScript)

(fn SetupNewGameSession
  (params (New%20Game :type Boolean) (Skip%20Lab%20Room :type Boolean))
  (bind _as_life_vr_character (Variables|Default|GetAs%20Life%20VR%20Character))
  (if New%20Game
    (if Skip%20Lab%20Room
      (Variables|Default|SetRoomIndex 1)
      (else
        (Variables|Default|SetRoomIndex 0)))
    (bind _returnvalue (Game|SpawnActorfromClass (Utilities|Array|Get(acopy) (Variables|GameSession|GetRoomsToPlay) (Variables|Default|GetRoomIndex)) (Math|Transform|MakeTransform "0, 0, 0" "0, 0, 0" "1.000000,1.000000,1.000000") "Undefined" "MultiplyWithRoot" 0 0))
    (bind _output_get (Variables|GameSession|SetCurrentRoom _returnvalue))
    (Variables|TimerManagement|SetTimerMinutes (Variables|/Script/EscapeGame.Room|GetAvailableTimeToResolve _output_get))
    ;[0.05469 0.05469 0.05469] Move player to the right room
    (Transformation|SetWorldTransform (Variables|/Script/VRExpansionPlugin.VRCharacter|GetVRRootReference _as_life_vr_character) (Transformation|GetWorldTransform (Variables|/Script/EscapeGame.Room|GetPlayerSpawn (Variables|GameSession|GetCurrentRoom))) false true)
    (Class|VRBaseCharacterMovementComponent|PerformMoveActionSetRotation (Variables|/Script/VRExpansionPlugin.VRBaseCharacter|GetVRMovementReference _as_life_vr_character) (.yaw (.Rotation (Math|Transform|BreakTransform (Transformation|GetWorldTransform (Variables|/Script/EscapeGame.Room|GetPlayerSpawn (Variables|GameSession|GetCurrentRoom)))))) "VRMOVEACTION_Velocity_None" false false false)
    (bind _returnvalue_2 (Actor|GetActorOfClass "/Game/UI/WBP_InteractableWidget.WBP_InteractableWidget_C"))
    (Actor|DestroyActor _returnvalue_2)
    (EventDispatchers|BindEventtoOnRoomSucceeded (Variables|GameSession|GetCurrentRoom) (EventDispatchers|CreateEvent :!event HandleRoomSucceeded))
    (else
      (Development|PrintString "")
      (CallFunction|LoadSavetoGameSession))))

(fn LoadSavetoGameSession
  (bind _savedata (Variables|GameSave|GetSaveData))
  (Utilities|IsValid _savedata
    (:Is%20Valid
      (Development|PrintString "Loading screen...")
      (bind _currentroom (Default|GetCurrentRoom _savedata))
      (Variables|GameSession|SetCurrentRoom _currentroom))))

(fn SaveGametoPersitentDataSave
  (Default|SaveGameSession (Variables|GameSave|GetSaveData) (Variables|GameSession|GetTeleportationEnabled) (Variables|GameSession|GetCurrentRoom) (Utilities|Array|MakeArray 0)))

(fn DefineRoomstoPlay
  ;[0.005208 0.005208 0.005208 1 12] Add parameters to select rooms depending oon parameteres
  ;[0.005208 0.005208 0.005208] TODO Add number of room logix
  (Utilities|Array|AddUnique (Variables|GameSession|GetRoomsToPlay) (.OutItem (Utilities|Array|Random (Variables|Default|GetAvailable%20Rooms%20Type)))))

(fn HandleRoomSucceeded
  (bind _generalgm_debug (Variables|DEBUG|GetGeneralGM%20Debug))
  (Development|PrintString "GM : Handle room succeed" _generalgm_debug _generalgm_debug))