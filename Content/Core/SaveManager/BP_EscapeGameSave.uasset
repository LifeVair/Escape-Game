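; BP_EscapeGameSave is the save object for an escape game, holding the partner-mode setting and session state: teleportation flag, current room, playable rooms and save time.
; SaveGameSession stamps the time and writes itself to the "PersistentData" slot, setting SessionSaveExists only after that write returns.
; SaveGameSettings and ResetSave change variables in memory only; reset clears the session but keeps partner mode.
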(fn SetPartnerModeEnabled
  (params (PartnerMode :type Boolean))
  (Variables|GameSettings|SetPartnerModeEnabled PartnerMode))

(fn GetPartnerModeEnabled
  (return (Variables|GameSettings|GetPartnerModeEnabled)))

(fn SetTeleportationEnabled
  (params (TeleportationEnabled :type Boolean))
  (Variables|GameSession|SetTeleportationEnabled TeleportationEnabled))

(fn GetTeleportationEnabled
  (return (Variables|GameSession|GetTeleportationEnabled)))

(fn SaveGameSettings
  (params (PartnerModeEnabled :type Boolean))
  (Variables|GameSettings|SetPartnerModeEnabled PartnerModeEnabled))

(fn SaveGameSession
  (params (Teleportation%20Enabled :type Boolean) (Current%20room%20 :type Room%20Object%20Reference) (Rooms :type Array%20of%20Room%20Object%20References))
  (Variables|GameSession|SetTeleportationEnabled Teleportation%20Enabled)
  (Variables|GameSession|SetCurrentRoom Current%20room%20)
  (Variables|GameSession|SetPlayable%20Rooms Rooms)
  (Variables|GameSession|SetSave%20Time (Math|DateTime|Now))
  (bind _returnvalue (SaveGame|SaveGametoSlot self "PersistentData"))
  (if _returnvalue
    (Variables|GameSession|SetSession%20Save%20Exists true)
    (else
      (Development|PrintString 0 "Error : Unable to save data in persistent data" true true "(R=1.000000,G=0.000000,B=0.007207,A=1.000000)" 1e+01)
      (Variables|GameSession|SetSession%20Save%20Exists false))))

(fn SetCurrentRoom
  (params (Current%20Room :type Room%20Object%20Reference))
  (Variables|GameSession|SetCurrentRoom Current%20Room))

(fn GetCurrentRoom
  (return (Variables|GameSession|GetCurrentRoom)))

(fn ResetSave
  (Variables|GameSession|SetSave%20Time "")
  (Utilities|Array|Clear (Variables|GameSession|GetPlayable%20Rooms))
  (Variables|GameSession|SetCurrentRoom 0)
  (Variables|GameSession|SetTeleportationEnabled false)
  (Variables|GameSession|SetSession%20Save%20Exists false))

(fn GameSessionExists
  (return (Variables|GameSession|GetSession%20Save%20Exists)))